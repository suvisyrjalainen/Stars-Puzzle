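; Laser emitter actor that traces a bouncing, branching beam from its forward vector every tick.
; ShootBeam line-traces, records each segment as a point pair, and calls LaserActivated.OnLaserHit on actors hit via tagged components.
; It recurses along each returned direction, ignoring the actor just hit, within remaining distance and bounce limits.
; The collected positions feed a Niagara array before the system resets, with beam color set in the construction script.
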(event EventTick
  (params (DeltaSeconds :type Float%20%28single-precision%29))
  (Utilities|Array|Clear (Variables|Default|GetBeam%20Positions))
  (CallFunction|ShootBeam (Transformation|GetWorldLocation (Variables|Default|GetLaser%20Beam)) (Transformation|GetActorForwardVector) self (Variables|Default|GetMax%20Distance) (Variables|Default|GetMax%20Bounces))
  (Class|NiagaraDataInterfaceArrayFunctionLibrary|SetNiagaraArrayPosition (Variables|Default|GetLaser%20Beam) "Positions" (Variables|Default|GetBeam%20Positions))
  (Niagara|ResetSystem (Variables|Default|GetLaser%20Beam)))

(fn ConstructionScript
  (Effects|Components|ParticleSystem|SetColorParameter (Variables|Default|GetLaser%20Beam) "Color" (Variables|Default|GetBeam%20Color)))

(fn ShootBeam
  (params (Start :type Vector) (Direction :type Vector) (Ignored%20Actor :type Actor%20Object%20Reference) (Max%20Distance :type Float%20%28double-precision%29) (Max%20Bounces :type Integer))
  (bind _returnvalue (- Max%20Bounces 1))
  (bind (_outhit _returnvalue_2) (Collision|LineTraceByChannel Start (|(start+(normal*distance)) Start Direction Max%20Distance) "TraceTypeQuery3" false (Utilities|Array|MakeArray Ignored%20Actor) "None" false))
  (|Addpositionstobeam (.TraceStart (Collision|BreakHitResult _outhit)) (Math|Vector|SelectVector (.ImpactPoint (Collision|BreakHitResult _outhit)) (.TraceEnd (Collision|BreakHitResult _outhit)) _returnvalue_2))
  (|Checkrecursionlimits (- Max%20Distance (.Distance (Collision|BreakHitResult _outhit))) _returnvalue _returnvalue_2 (.HitComponent (Collision|BreakHitResult _outhit)))
  (bind _aslaser_activated (Utilities|Casting|CastToLaserActivated (.HitActor (Collision|BreakHitResult _outhit))))
  (bind _outgoing_laser_directions (Default|OnLaserHit _aslaser_activated Direction (.ImpactNormal (Collision|BreakHitResult _outhit))))
  (bind _valuepin (Utilities|Set|ForEachLoop(Set) _outgoing_laser_directions)
    (:then
      (CallFunction|ShootBeam (Math|Vector|SelectVector (.ImpactPoint (Collision|BreakHitResult _outhit)) (.TraceEnd (Collision|BreakHitResult _outhit)) _returnvalue_2) _valuepin (.HitActor (Collision|BreakHitResult _outhit)) (- Max%20Distance (.Distance (Collision|BreakHitResult _outhit))) _returnvalue))))