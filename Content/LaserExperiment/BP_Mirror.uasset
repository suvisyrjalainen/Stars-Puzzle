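; BP_Mirror is a rotatable mirror turret in the laser experiment.
; Its Rotate function adds an amount to a stored Rotation, wrapped to 360 degrees.
; It then sets the Turret component's relative yaw, snapped to the nearest multiple of RotationStepSize.
; The construction script is empty.
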(fn ConstructionScript)

(fn Rotate
  (params (Amount :type Float%20%28double-precision%29))
  (bind _rotationstepsize (Variables|Default|GetRotationStepSize))
  (Variables|Default|SetRotation (Math|Float|%(Float) (+ Amount (Variables|Default|GetRotation)) 3.6e+02))
  (Transformation|SetRelativeRotation (Variables|Default|GetTurret) (Math|Rotator|MakeRotator 0.0 0.0 (* (Math|Float|Round (/ (Math|Float|%(Float) (+ Amount (Variables|Default|GetRotation)) 3.6e+02) _rotationstepsize)) _rotationstepsize)) false false))